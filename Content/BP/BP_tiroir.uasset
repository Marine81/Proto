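; Interactable drawer that opens a keypad widget (WBP_Digicode) posing an arithmetic puzzle.
; A box overlap tracks whether the first-person character is near; Interact then creates the widget once and switches to UI-only input with a cursor.
; IndexTiroir selects each drawer's hard-coded calculation, answer and spawn location, passed to the widget along with the drawer itself.
; ResetTiroir destroys actors in the Platforme array, clearing it inside the loop.
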(event OnComponentBeginOverlap(Box)
  (params (OverlappedComponent :type Primitive%20Component%20Object%20Reference) (OtherActor :type Actor%20Object%20Reference) (OtherComp :type Primitive%20Component%20Object%20Reference) (OtherBodyIndex :type Integer) (bFromSweep :type Boolean) (SweepResult :type Hit%20Result%20Structure%20%28by%20ref%29))
  (Utilities|Casting|CastToBP_FirstPersonCharacter OtherActor)
  (Variables|Default|SetjoueurProche true))

(event OnComponentEndOverlap(Box)
  (params (OverlappedComponent :type Primitive%20Component%20Object%20Reference) (OtherActor :type Actor%20Object%20Reference) (OtherComp :type Primitive%20Component%20Object%20Reference) (OtherBodyIndex :type Integer))
  (Utilities|Casting|CastToBP_FirstPersonCharacter OtherActor)
  (Variables|Default|SetjoueurProche false))

(event EventBeginPlay)

(event Collision|EventActorBeginOverlap
  (params (OtherActor :type Actor%20Object%20Reference)))

(event EventInteract
  (bind _returnvalue (Game|GetPlayerController 0))
  (bind _index_tiroir (Variables|Default|Getindex%20tiroir))
  (if (Variables|Default|GetjoueurProche)
    (if (not (Variables|Default|GetestOuvert))
      (Utilities|IsValid (Variables|Default|Getwidgetactif)
        (:Is%20Not%20Valid
          (bind _returnvalue_2 (UserInterface|CreateWidget "/Game/ui/WBP_Digicode.WBP_Digicode_C" 0 self (Utilities|Select :Index _index_tiroir :Option%200 "163.000000,2025.000000,80.000000" :Option%201 "145.000000,2723.000000,108.000000" :Option%202 "-391.000000,2724.000000,238.000000" :Option%203 "-383.000000,2200.000000,355.000000" :Option%204 "-1029.000000,2200.000000,496.000000" :Option%205 "-110.000000,302.000000,164.000000" :Option%206 "522.000000,174.000000,296.000000" :Option%207 "522.000000,717.000000,438.000000" :Option%208 "530.000000,1246.000000,576.000000" :Option%209 "-1641.000000,1972.000000,637.000000" :Option%2010 "-1438.000000,1465.000000,744.000000" :Option%2011 "406.000000,1824.000000,708.000000" :Option%2012 "419.000000,1290.000000,825.000000" :Option%2013 "-1684.000000,844.000000,854.000000" :Option%2014 "-1202.000000,844.000000,924.000000") (Utilities|Select :Index _index_tiroir :Option%200 "2+2" :Option%201 "55-30" :Option%202 "100-64" :Option%203 "236+24" :Option%204 "345+199" :Option%205 "8*8" :Option%206 "240/8" :Option%207 "6*9/3" :Option%208 "80*3/6" :Option%209 "700-245" :Option%2010 "278+22" :Option%2011 "25²" :Option%2012 "10²*2²" :Option%2013 "45+28+12" :Option%2014 "78-25+7") (Utilities|Select :Index _index_tiroir :Option%200 "4" :Option%201 "25" :Option%202 "36" :Option%203 "260" :Option%204 "544" :Option%205 "64" :Option%206 "30" :Option%207 "18" :Option%208 "40" :Option%209 "455" :Option%2010 "300" :Option%2011 "625" :Option%2012 "400" :Option%2013 "85" :Option%2014 "60")))
          (bind _output_get (Variables|Default|Setwidgetactif _returnvalue_2))
          (Variables|Default|SetestOuvert true)
          (UserInterface|Viewport|AddtoViewport _output_get 0)
          (Widget|SetKeyboardFocus _output_get)
          (Default|InitDIgicode _returnvalue_2)
          (Input|SetInputModeUIOnly _returnvalue 0 "DoNotLock" false)
          (Variables|/Script/Engine.PlayerController|SetbShowMouseCursor _returnvalue true))))))

(fn ConstructionScript)

(fn ResetTiroir
  (bind _platforme (Variables|Default|Getplatforme))
  (for _array_element _platforme
    (Actor|DestroyActor _array_element)
    (Utilities|Array|Clear _platforme)))