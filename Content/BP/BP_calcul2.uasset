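; BP_calcul2 is an interactable actor that opens a digicode (keypad) widget for the player.
; A Box overlap tracks whether the first-person character is nearby.
; On Interact, if the player is near and EstOuvert is false, it creates WBP_Digicode2 with itself as Codecible, unless one is already valid.
; It then shows the widget, switches input to UI only and displays the mouse cursor.
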(event OnComponentBeginOverlap(Box)
  (params (OverlappedComponent :type Primitive%20Component%20Object%20Reference) (OtherActor :type Actor%20Object%20Reference) (OtherComp :type Primitive%20Component%20Object%20Reference) (OtherBodyIndex :type Integer) (bFromSweep :type Boolean) (SweepResult :type Hit%20Result%20Structure%20%28by%20ref%29))
  (Utilities|Casting|CastToBP_FirstPersonCharacter OtherActor)
  (Variables|Default|SetjoueurProche true))

(event OnComponentEndOverlap(Box)
  (params (OverlappedComponent :type Primitive%20Component%20Object%20Reference) (OtherActor :type Actor%20Object%20Reference) (OtherComp :type Primitive%20Component%20Object%20Reference) (OtherBodyIndex :type Integer))
  (Utilities|Casting|CastToBP_FirstPersonCharacter OtherActor)
  (Variables|Default|SetjoueurProche false))

(event EventBeginPlay)

(event Collision|EventActorBeginOverlap
  (params (OtherActor :type Actor%20Object%20Reference)))

(event EventTick
  (params (DeltaSeconds :type Float%20%28single-precision%29)))

(event EventInteract
  (bind _returnvalue (Game|GetPlayerController 0))
  (if (Variables|Default|GetjoueurProche)
    (if (not (Variables|Default|GetestOuvert))
      (Utilities|IsValid (Variables|Default|Getnouveauwidgetactif)
        (:Is%20Not%20Valid
          (bind _returnvalue_2 (UserInterface|CreateWidget "/Game/ui/WBP_Digicode2.WBP_Digicode2_C" 0 self))
          (bind _output_get (Variables|Default|Setnouveauwidgetactif _returnvalue_2))
          (UserInterface|Viewport|AddtoViewport _output_get 0)
          (Input|SetInputModeUIOnly _returnvalue 0 "DoNotLock" false)
          (Variables|/Script/Engine.PlayerController|SetbShowMouseCursor _returnvalue true))))))

(fn ConstructionScript)