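; BP_Teleport is an overlap trigger that sends the player back to PointDepart and resets the drawer (tiroir) game state.
; On any actor overlap, it sets EstOuvert to true on every valid BP_tiroir.
; After each drawer and again when the loop completes, it moves player 0's BP_FirstPersonCharacter, then has GM_tiroir reset the drawers and destroy all platforms.
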(event EventBeginPlay)

(event Collision|EventActorBeginOverlap
  (params (OtherActor :type Actor%20Object%20Reference))
  (bind _returnvalue (Game|GetPlayerCharacter 0))
  (Actor|GetAllActorsOfClass "/Game/BP/BP_tiroir.BP_tiroir_C")
  (for _array_element 0
    (Utilities|IsValid _array_element
      (:Is%20Valid
        (Variables|/Game/BP/BP_tiroir.BP_tiroir_C|SetestOuvert _array_element true)
        (Utilities|Casting|CastToBP_FirstPersonCharacter _returnvalue)
        (Transformation|SetActorLocation _returnvalue (Variables|Default|GetpointDepart) false false)
        (bind _asgm_tiroir (Utilities|Casting|CastToGM_tiroir (Game|GetGameMode)))
        (Default|ResetTiroir _asgm_tiroir)
        (Default|DestroyAllPlatforme _asgm_tiroir))))
  (Utilities|Casting|CastToBP_FirstPersonCharacter _returnvalue)
  (Transformation|SetActorLocation _returnvalue (Variables|Default|GetpointDepart) false false)
  (bind _asgm_tiroir_2 (Utilities|Casting|CastToGM_tiroir (Game|GetGameMode)))
  (Default|ResetTiroir _asgm_tiroir_2)
  (Default|DestroyAllPlatforme _asgm_tiroir_2))

(event EventTick
  (params (DeltaSeconds :type Float%20%28single-precision%29)))

(fn ConstructionScript)