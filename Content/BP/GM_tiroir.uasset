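; GM_tiroir, apparently a game mode, manages spawned platforms and the state of drawer actors (BP_tiroir).
; Its spawn event creates a BP_Platforme at a given location and stores it in an array.
; A cleanup event destroys every stored platform without clearing the array.
; A reset event finds all drawers and clears their active widget, open and player-nearby states, with debug prints in both cleanup and reset.
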(event Custom|spawnPlatforme
  (params (Spawn%20Transform%20Location :type Vector))
  (bind _returnvalue (Game|SpawnActorfromClass "/Game/BP/BP_Platforme.BP_Platforme_C" (Math|Transform|MakeTransform Spawn%20Transform%20Location "0, 0, 0" "1.000000,1.000000,1.000000") "Undefined" "MultiplyWithRoot" 0 0))
  (Utilities|Array|Add (Variables|Default|Getplatforme) _returnvalue))

(event Custom|destroyAllPlatforme
  (bind _platforme (Variables|Default|Getplatforme))
  (Development|PrintString (Utilities|String|Append "delete platform: " (Utilities|String|ToString(Integer) (Utilities|Array|Length _platforme))))
  (for _array_element _platforme
    (Actor|DestroyActor _array_element)))

(event Custom|reset%20tiroir
  (bind _outactors (Actor|GetAllActorsOfClass "/Game/BP/BP_tiroir.BP_tiroir_C"))
  (Development|PrintString (Utilities|String|ToString(Integer) (Utilities|Array|Length _outactors)))
  (for _array_element _outactors
    (Variables|/Game/BP/BP_tiroir.BP_tiroir_C|Setwidgetactif _array_element 0)
    (Variables|/Game/BP/BP_tiroir.BP_tiroir_C|SetestOuvert _array_element false)
    (Variables|/Game/BP/BP_tiroir.BP_tiroir_C|SetjoueurProche _array_element false)))

(fn ConstructionScript)