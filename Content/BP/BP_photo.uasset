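; BP_photo is an interactable photo actor that opens a WBP_Photo screen while its clue has not been retrieved (IndiceRecuperer).
; On Interact, it creates the widget only if none is valid, passing itself as the target frame (CadreCible).
; It then adds the widget to the viewport, switches input to UI only and shows the mouse cursor.
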(event EventBeginPlay)

(event Collision|EventActorBeginOverlap
  (params (OtherActor :type Actor%20Object%20Reference)))

(event EventTick
  (params (DeltaSeconds :type Float%20%28single-precision%29)))

(event EventInteract
  (bind _returnvalue (Game|GetPlayerController 0))
  (if (not (Variables|Default|GetIndiceRecuperer))
    (Utilities|IsValid (Variables|Default|GetwidgetPhoto)
      (:Is%20Not%20Valid
        (bind _returnvalue_2 (UserInterface|CreateWidget "/Game/ui/WBP_Photo.WBP_Photo_C" 0 self))
        (bind _output_get (Variables|Default|SetwidgetPhoto _returnvalue_2))
        (UserInterface|Viewport|AddtoViewport _output_get 0)
        (Input|SetInputModeUIOnly _returnvalue 0 "DoNotLock" false)
        (Variables|/Script/Engine.PlayerController|SetbShowMouseCursor _returnvalue true)))))

(fn ConstructionScript)